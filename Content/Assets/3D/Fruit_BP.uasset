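; A sliceable fruit actor that rolls a random score within its min and max when play begins.
; Its Sliced event orients the sliced-fruit parent along the blade's motion, using a fixed relative rotation if the blade barely moved.
; It disables the whole fruit's collision, then a tick later hides it and shows the top and bottom halves as simulating physics bodies.
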(event `self.ReceiveBeginPlay`
  (set `self.ScoreOnFruit` (`KismetMathLibrary.RandomIntegerInRange` (`self.ScoreMinOnFruit`) (`self.ScoreMaxOnFruit`))))

(event `Sliced`
  (params (previousBladePosition :type "Vector Structure (by ref)") (currentBladePosition :type "Vector Structure (by ref)"))
  (bind _parentfruitsliced (`self.ParentFruitSliced`))
  (bind _fruit_whole (`self.Fruit_Whole`))
  (bind _fruit_sliced_top (`self.Fruit_Sliced_Top`))
  (if (== previousBladePosition currentBladePosition :`ErrorTolerance` 0.2)
    (`SceneComponent.K2_SetRelativeRotation` _parentfruitsliced (struct :`Pitch` 90.0) false false)
    (else
      (`SceneComponent.K2_SetWorldRotation` _parentfruitsliced (`KismetMathLibrary.FindLookAtRotation` previousBladePosition currentBladePosition) false false)))
  (`PrimitiveComponent.SetCollisionProfileName` _fruit_whole "NoCollision" true)
  (`KismetSystemLibrary.DelayUntilNextTick`)
  (`SceneComponent.SetVisibility` _fruit_whole false false)
  (`SceneComponent.SetVisibility` _fruit_sliced_top true false)
  (`SceneComponent.SetVisibility` (`self.Fruit_Sliced_Bottom`) true false)
  (`PrimitiveComponent.SetSimulatePhysics` _fruit_sliced_top true)
  (`PrimitiveComponent.SetSimulatePhysics` (`self.Fruit_Sliced_Bottom`) true))

(fn `UserConstructionScript`)