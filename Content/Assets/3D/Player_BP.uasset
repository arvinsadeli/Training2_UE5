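; Player Blueprint for a fruit-slicing game, where a mouse-driven blade cuts fruit and bombs and tracks score.
; On BeginPlay it adds the Enhanced Input context, shows the cursor and creates the gameplay HUD.
; Holding left mouse teleports the blade to the cursor trace hit, recording previous and delayed current positions; release or a miss moves it far away.
; Sphere overlaps call Sliced, passing blade positions to fruit and updating score.
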(event `self.ReceiveBeginPlay`
  (message `EnhancedInputSubsystemInterface.AddMappingContext` (pcsubsystem `EnhancedInputLocalPlayerSubsystem` (`GameplayStatics.GetPlayerController` 0)) "/Game/ThirdPerson/IMC/Player_IMC.Player_IMC" 5 (struct))
  (set `PlayerController.bShowMouseCursor` true (`GameplayStatics.GetPlayerController` 0))
  (bind _returnvalue (`|CreateWidget` "/Game/ThirdPerson/Gameplay_Widget.Gameplay_Widget_C"))
  (bind _output_get (set `self.GameplayWidget` _returnvalue))
  (`UserWidget.AddToViewport` _output_get 0)
  (bind _output_get_2 (set `self.score` (`self.score`)))
  (`/Game/ThirdPerson/Gameplay_Widget.SetScoreUI` (`self.GameplayWidget`) _output_get_2))

(event `EnhancedInput|/Game/ThirdPerson/IMC/LeftMouseButton_IA`
  (params (ActionValue :type Boolean) (ElapsedSeconds :type "Float (double-precision)") (TriggeredSeconds :type "Float (double-precision)") (InputAction :type "InputAction Object Reference" :default "/Game/ThirdPerson/IMC/LeftMouseButton_IA.LeftMouseButton_IA"))
  (bind _hitresult (`PlayerController.GetHitResultUnderCursorByChannel` (`GameplayStatics.GetPlayerController` 0) "TraceTypeQuery1" true))
  (:`Triggered`
    (if (`GameplayStatics.BreakHitResult` _hitresult)
      (set `self.previousBladePosition` (`SceneComponent.K2_GetComponentLocation` (`self.Blade`)))
      (`SceneComponent.K2_SetWorldLocation` (`self.Blade`) (`.Location` (`GameplayStatics.BreakHitResult` _hitresult)) false true)
      (`KismetSystemLibrary.Delay` 1.0)
      (set `self.CurrentBladePosition` (`SceneComponent.K2_GetComponentLocation` (`self.Blade`)))
      (else
        (`SceneComponent.K2_SetRelativeLocation` (`self.Blade`) (-10000000.0 0.0 0.0) false true :!label _label))))
  (:`Completed`
    (goto _label)))

(event `self.Sphere.OnComponentBeginOverlap`
  (params (OverlappedComponent :type "PrimitiveComponent Object Reference") (OtherActor :type "Actor Object Reference") (OtherComp :type "PrimitiveComponent Object Reference") (OtherBodyIndex :type Integer) (bFromSweep :type Boolean) (SweepResult :type "HitResult Structure (by ref)"))
  (`KismetSystemLibrary.PrintString` (`KismetSystemLibrary.GetDisplayName` OverlappedComponent))
  (bind _asfruit_bp (cast `/Game/Assets/3D/Fruit_BP` OtherActor)
    (:`then`
      (`/Game/Assets/3D/Fruit_BP.Sliced` _asfruit_bp (`self.previousBladePosition`) (`self.CurrentBladePosition`))
      (bind _output_get (set `self.score` (+ (stale _output_get) (`/Game/Assets/3D/Fruit_BP.ScoreOnFruit` _asfruit_bp))))
      (`/Game/ThirdPerson/Gameplay_Widget.SetScoreUI` (`self.GameplayWidget`) _output_get))
    (:`CastFailed`
      (bind _asbomb_bp (cast `/Game/Assets/3D/Bomb_BP` OtherActor))
      (`/Game/Assets/3D/Bomb_BP.Sliced` _asbomb_bp))))

(fn `UserConstructionScript`)