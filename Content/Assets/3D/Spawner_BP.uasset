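; Spawner actor that continuously spawns fruit or bomb actors at random positions along the Y axis around its location.
; From BeginPlay, a Spawn event picks Bomb_BP or Fruit_BP by a percentage chance, then calls itself after a random delay.
; Tick draws debug boxes at plus and minus the Y radius, using absolute world Y rather than an offset from the actor.
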(event `self.ReceiveBeginPlay`
  (`self.Spawn`))

(event `self.ReceiveTick`
  (params (DeltaSeconds :type "Float (single-precision)"))
  (bind (_returnvalue_x _returnvalue_y _returnvalue_z) (`KismetMathLibrary.BreakVector` (`self.K2_GetActorLocation`)))
  (bind __spawnradiusy (`self. SpawnRadiusY`))
  (`KismetSystemLibrary.DrawDebugBox` (`KismetMathLibrary.MakeVector` _returnvalue_x (* __spawnradiusy -1.0) _returnvalue_z) (1.0 1.0 1.0) (struct :`G` 0.521569 :`B` 1.0 :`A` 1.0) (struct) 5.0 5.0)
  (`KismetSystemLibrary.DrawDebugBox` (`KismetMathLibrary.MakeVector` _returnvalue_x __spawnradiusy _returnvalue_z) (1.0 1.0 1.0) (struct :`G` 0.521569 :`B` 1.0 :`A` 1.0) (struct) 5.0 5.0))

(event `Spawn`
  (bind __spawnradiusy (`self. SpawnRadiusY`))
  (`|SpawnActorFromClass` (select `bool` (<= (`KismetMathLibrary.RandomIntegerInRange` 0 100) (`self.bombSpawnChance`)) :`false` "/Game/Assets/3D/Fruit_BP.Fruit_BP_C" :`true` "/Game/Assets/3D/Bomb_BP.Bomb_BP_C" :!type "Actor Class Reference") (`KismetMathLibrary.MakeTransform` (+ (`self.K2_GetActorLocation`) (`KismetMathLibrary.MakeVector` 0.0 (`KismetMathLibrary.RandomFloatInRange` (* __spawnradiusy -1.0) __spawnradiusy)))) "Undefined" "MultiplyWithRoot" null null)
  (`KismetSystemLibrary.RetriggerableDelay` (`KismetMathLibrary.RandomFloatInRange` (`self.MinDuration`) (`self.MaxDuration`)))
  (`self.Spawn`))

(fn `UserConstructionScript`)